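; Master planet actor that builds a sphere of a given radius in meters and scatters static meshes, likely grass, over its surface.
; The construction script scales the planet mesh from its bounds, then adds randomly scaled components, each randomly rotated at the center and pushed along local Z to just below the radius.
; GetSurfaceAndNormal projects a location onto the sphere but is not called here; a line-trace scatter is left disconnected.
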(event EventBeginPlay)

(event Collision|EventActorBeginOverlap
  (params (OtherActor :type Actor%20Object%20Reference)))

(event EventTick
  (params (DeltaSeconds :type Float%20%28single-precision%29)))

(fn ConstructionScript
  (bind _output_get (Variables|Default|SetRadiusInUntis (* (Variables|Default|GetRadiusInMeters) 1e+02)))
  (Transformation|SetWorldScale3D (Variables|Default|GetPlanetUV8) (Math|Conversions|ToVector(Float) (/ _output_get (.x (.BoxExtent (Collision|GetComponentBounds (Variables|Default|GetPlanetUV8)))))))
  (CallFunction|SpawnActorSurface))

(fn GetSurfaceandNormal
  (params (Location :type Vector))
  (bind _returnvalue (Transformation|GetActorLocation))
  (bind _returnvalue_2 (- Location _returnvalue))
  (bind _returnvalue_3 (Math|Vector|Normalize _returnvalue_2))
  (return _returnvalue_3 (+ (* _returnvalue_3 (Variables|Default|GetRadiusInUntis)) (Transformation|GetActorLocation))))

(fn SpawnActorSurface
  (bind _smeshscalemax (Variables|Default|GetSmeshScaleMax))
  (bind _returnvalue (Math|Random|RandomFloatinRange 1.0 _smeshscalemax))
  (for _index (range 0 (Variables|Default|GetMaxGrass))
    (bind _returnvalue_2 (AddComponent|AddStaticMeshComponent true (Math|Transform|MakeTransform (Transformation|GetWorldLocation (Variables|Default|GetPlanetUV8)))))
    (Transformation|SetWorldRotation _returnvalue_2 (Math|Random|RandomRotator false) false false)
    (Transformation|AddLocalOffset _returnvalue_2 (Math|Vector|MakeVector 0.0 0.0 (- (Variables|Default|GetRadiusInUntis) 5e+02)) false false)
    (Transformation|SetWorldScale3D _returnvalue_2 (Math|Vector|MakeVector _returnvalue _returnvalue _returnvalue))))